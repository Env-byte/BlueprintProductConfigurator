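; Speaker finish configurator that cycles the look of a set of speakers through preset options.
; InitSpeakerLogic stores the speaker array, and each Clicked function advances its own wrapping index to select a preset for cabinet, drivers, accents or screen.
; Setter functions apply it to components each speaker exposes through getters.
; Cabinet, tweeter and woofer, and accent and feet finishes swap materials, while screen colour sets a "Color" vector parameter.
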(event EventBeginPlay)

(event Collision|EventActorBeginOverlap
  (params (OtherActor :type Actor%20Object%20Reference)))

(event EventTick
  (params (DeltaSeconds :type Float%20%28single-precision%29)))

(fn ConstructionScript)

(fn CabinetClicked
  (bind _output_get (Variables|Cabinet|SetCabinetIndex (Math|Integer|%(Integer) (+ (Variables|Cabinet|GetCabinetIndex) 1) (Variables|Cabinet|GetCabinetMaxIndex))))
  (switch int _output_get
    (:0
      (SetMaterial|SetCabinetMaterial "/Game/Spkrs/m/BlkGld_Cab.BlkGld_Cab"))
    (:1
      (SetMaterial|SetCabinetMaterial "/Game/Spkrs/m/EbStl_Cab.EbStl_Cab"))
    (:2
      (SetMaterial|SetCabinetMaterial "/Game/Spkrs/m/TkBlk_Cab.TkBlk_Cab"))
    (:3
      (SetMaterial|SetCabinetMaterial "/Game/Spkrs/m/WalSlv_Cab.WalSlv_Cab"))
    (:4
      (SetMaterial|SetCabinetMaterial "/Game/Spkrs/m/WhtCp_Cab.WhtCp_Cab"))))

(fn SetCabinetMaterial
  (params (Material :type Material%20Object%20Reference))
  (for _array_element (Variables|Default|GetSpeakerArray)
    (bind _cabinette (Default|GetCabinetComponent _array_element))
    (Rendering|Material|SetMaterial _cabinette 0 Material)))

(fn InitSpeakerLogic
  (params (SpeakerArrayIn :type Array%20of%20BP%20Speaker%20Object%20References))
  (Variables|Default|SetSpeakerArray SpeakerArrayIn))

(fn SpeakerClicked
  (bind _output_get (Variables|Speaker|SetSpeakerIndex (Math|Integer|%(Integer) (+ (Variables|Speaker|GetSpeakerIndex) 1) (Variables|Speaker|GetSpeakerIndexMax))))
  (switch int _output_get
    (:0
      (SetMaterial|SetSpeakerMaterials "/Game/Spkrs/m/BlkGld_Twt.BlkGld_Twt" "/Game/Spkrs/m/BlkGld_Wof.BlkGld_Wof"))
    (:1
      (SetMaterial|SetSpeakerMaterials "/Game/Spkrs/m/TkBlk_Twt.TkBlk_Twt" "/Game/Spkrs/m/TkBlk_Wof.TkBlk_Wof"))
    (:2
      (SetMaterial|SetSpeakerMaterials "/Game/Spkrs/m/WalSlv_Twt.WalSlv_Twt" "/Game/Spkrs/m/WalSlv_Wof.WalSlv_Wof"))
    (:3
      (SetMaterial|SetSpeakerMaterials "/Game/Spkrs/m/WhtCp_Twt.WhtCp_Twt" "/Game/Spkrs/m/WhtCp_Wof.WhtCp_Wof"))))

(fn SetSpeakerMaterials
  (params (Tweeter%20Material%20In :type Material%20Object%20Reference) (Woofer%20Material%20In :type Material%20Object%20Reference))
  (for _array_element (Variables|Default|GetSpeakerArray)
    (bind (_woofers _horntweeter) (Default|GetSpeakerComponents _array_element))
    (Utilities|FlowControl|Sequence
      (:then_0
        (Rendering|Material|SetMaterial _horntweeter 0 Tweeter%20Material%20In))
      (:then_1
        (Rendering|Material|SetMaterial _woofers 0 Woofer%20Material%20In)))))

(fn AccentClicked
  (bind _output_get (Variables|Accent|SetAccentIndex (Math|Integer|%(Integer) (+ (Variables|Accent|GetAccentIndex) 1) (Variables|Accent|GetAccentIndexMax))))
  (switch int _output_get
    (:0
      (SetMaterial|SetAccentMaterials "/Game/Spkrs/m/BlkGld_Ft.BlkGld_Ft" "/Game/Spkrs/m/BlkGld_Cab.BlkGld_Cab"))
    (:1
      (SetMaterial|SetAccentMaterials "/Game/Spkrs/m/EbStl_Ft.EbStl_Ft" "/Game/Spkrs/m/EbStl_Cab.EbStl_Cab"))
    (:2
      (SetMaterial|SetAccentMaterials "/Game/Spkrs/m/TkBlk_Ft.TkBlk_Ft" "/Game/Spkrs/m/TkBlk_Cab.TkBlk_Cab"))
    (:3
      (SetMaterial|SetAccentMaterials "/Game/Spkrs/m/WalSlv_Ft.WalSlv_Ft" "/Game/Spkrs/m/WalSlv_Cab.WalSlv_Cab"))
    (:4
      (SetMaterial|SetAccentMaterials "/Game/Spkrs/m/WhtCp_Ft.WhtCp_Ft" "/Game/Spkrs/m/WhtCp_Cab.WhtCp_Cab"))))

(fn SetAccentMaterials
  (params (Feet%20Material :type Material%20Object%20Reference) (Accent%20Material :type Material%20Object%20Reference))
  (for _array_element (Variables|Default|GetSpeakerArray)
    (bind (_feet_components _accent_components) (Default|GetAccentComponents _array_element))
    (Utilities|FlowControl|Sequence
      (:then_0
        (for _array_element_2 _feet_components
          (Rendering|Material|SetMaterial _array_element_2 0 Feet%20Material)))
      (:then_1
        (for _array_element_3 _accent_components
          (Rendering|Material|SetMaterial _array_element_3 0 Accent%20Material))))))

(fn ScreenClicked
  (bind _output_get (Variables|Screen|SetScreenIndex (Math|Integer|%(Integer) (+ (Variables|Screen|GetScreenIndex) 1) (Variables|Screen|GetScreenIndexMax))))
  (switch int _output_get
    (:0
      ;[1 1 1] Black
      (SetMaterial|SetScreenColour "0, 0, 0"))
    (:1
      ;[1 1 1] Gold
      (SetMaterial|SetScreenColour "0.144100,0.115500,0.032300"))
    (:2
      ;[1 1 1] Dark Grey
      (SetMaterial|SetScreenColour "0.890000,0.890000,0.890000"))
    (:3
      ;[1 1 1] White
      (SetMaterial|SetScreenColour "1.000000,1.000000,1.000000"))
    (:4
      ;[1 1 1] Dark Brown
      (SetMaterial|SetScreenColour "0.642000,0.023700,0.009300"))))

(fn SetScreenColour
  (params (colour :type Vector))
  (for _array_element (Variables|Default|GetSpeakerArray)
    (bind _screen (Default|GetScreenComponent _array_element))
    (Rendering|Material|SetVectorParameterValueonMaterials _screen "Color" colour)))