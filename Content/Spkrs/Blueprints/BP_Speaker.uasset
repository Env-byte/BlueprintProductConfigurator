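; BP_Speaker is a clickable speaker model made of cabinet, screen cover, woofer, horn tweeter, frame, plate and feet components.
; Component clicks are forwarded to a SpeakerLogic reference by part group: cabinet, screen, speakers or accents.
; InitSpeakerBP stores that reference and shows or hides the screen and frame based on CoverActive, ignoring collision when hidden.
; Getter functions expose each group's components.
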(event OnClicked(Woofers)
  (params (TouchedComponent :type Primitive%20Component%20Object%20Reference) (ButtonPressed :type Key%20Structure :default "None"))
  ;[1 1 1] Speakers clicked
  (Default|SpeakerClicked (Variables|Default|GetSpeaker%20Logic)))

(event OnClicked(AccentPlate)
  (params (TouchedComponent :type Primitive%20Component%20Object%20Reference) (ButtonPressed :type Key%20Structure :default "None"))
  ;[1 1 1] Accents clicked
  (Default|AccentClicked (Variables|Default|GetSpeaker%20Logic)))

(event OnClicked(Cabinette)
  (params (TouchedComponent :type Primitive%20Component%20Object%20Reference) (ButtonPressed :type Key%20Structure :default "None"))
  ;[1 1 1] Cabinet clicked
  (Default|CabinetClicked (Variables|Default|GetSpeaker%20Logic)))

(event OnClicked(Foot_BL)
  (params (TouchedComponent :type Primitive%20Component%20Object%20Reference) (ButtonPressed :type Key%20Structure :default "None"))
  ;[1 1 1] Accents clicked
  (Default|AccentClicked (Variables|Default|GetSpeaker%20Logic)))

(event OnClicked(Foot_BR)
  (params (TouchedComponent :type Primitive%20Component%20Object%20Reference) (ButtonPressed :type Key%20Structure :default "None"))
  ;[1 1 1] Accents clicked
  (Default|AccentClicked (Variables|Default|GetSpeaker%20Logic)))

(event OnClicked(Foot_FR)
  (params (TouchedComponent :type Primitive%20Component%20Object%20Reference) (ButtonPressed :type Key%20Structure :default "None"))
  ;[1 1 1] Accents clicked
  (Default|AccentClicked (Variables|Default|GetSpeaker%20Logic)))

(event OnClicked(Foot_FL)
  (params (TouchedComponent :type Primitive%20Component%20Object%20Reference) (ButtonPressed :type Key%20Structure :default "None"))
  ;[1 1 1] Accents clicked
  (Default|AccentClicked (Variables|Default|GetSpeaker%20Logic)))

(event OnClicked(Frame)
  (params (TouchedComponent :type Primitive%20Component%20Object%20Reference) (ButtonPressed :type Key%20Structure :default "None"))
  ;[1 1 1] Accents clicked
  (Default|AccentClicked (Variables|Default|GetSpeaker%20Logic)))

(event OnClicked(Screen)
  (params (TouchedComponent :type Primitive%20Component%20Object%20Reference) (ButtonPressed :type Key%20Structure :default "None"))
  ;[1 1 1] Screen clicked
  (Default|ScreenClicked (Variables|Default|GetSpeaker%20Logic)))

(event OnClicked(HornTweeter)
  (params (TouchedComponent :type Primitive%20Component%20Object%20Reference) (ButtonPressed :type Key%20Structure :default "None"))
  ;[1 1 1] Speakers clicked
  (Default|SpeakerClicked (Variables|Default|GetSpeaker%20Logic)))

(event EventBeginPlay)

(event Collision|EventActorBeginOverlap
  (params (OtherActor :type Actor%20Object%20Reference)))

(event EventTick
  (params (DeltaSeconds :type Float%20%28single-precision%29)))

(fn ConstructionScript)

(fn GetCabinetComponent
  (return (Variables|Default|GetCabinette)))

(fn InitSpeakerBP
  (params (Speaker%20Logic :type BP%20Speaker%20Logic%20Object%20Reference))
  (Utilities|FlowControl|Sequence
    (:then_0
      (Variables|Default|SetSpeaker%20Logic Speaker%20Logic))
    (:then_1
      ;[1 1 1] Check Cover Active
      (if (Variables|Default|GetCoverActive)
        ;;[0.04267 1 0] True
        (Rendering|SetVisibility (Variables|Default|GetScreen) true false)
        (Rendering|SetVisibility (Variables|Default|GetFrame) true false)
        (else
          ;;[1 0 0.02122] False
          (Rendering|SetVisibility (Variables|Default|GetScreen) false false)
          (Rendering|SetVisibility (Variables|Default|GetFrame) false false)
          (Collision|SetCollisionResponsetoAllChannels (Variables|Default|GetScreen) "ECR_Ignore")
          (Collision|SetCollisionResponsetoAllChannels (Variables|Default|GetFrame) "ECR_Ignore"))))))

(fn GetSpeakerComponents
  (return (Variables|Default|GetWoofers) (Variables|Default|GetHornTweeter)))

(fn GetAccentComponents
  (return (Utilities|Array|MakeArray (Variables|Default|GetFoot_FL) (Variables|Default|GetFoot_FR) (Variables|Default|GetFoot_BR) (Variables|Default|GetFoot_BL)) (Utilities|Array|MakeArray (Variables|Default|GetFrame) (Variables|Default|GetAccentPlate))))

(fn GetScreenComponent
  (return (Variables|Default|GetScreen)))